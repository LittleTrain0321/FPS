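; RU74 rifle actor for the player, handling automatic fire, recoil and magazine reloads.
; A looping timer spawns bullets at the muzzle socket, straight when aiming or cone-scattered otherwise, with paired arms and gun montages.
; Each shot triggers a timeline that nudges controller pitch and random yaw.
; Reload zeroes the magazine to block firing, picks empty or partial montages, and refills from reserve ammo when the gun montage completes.
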(event EventBeginPlay
  (bind _asbp_player (Utilities|Casting|CastToBP_Player (Game|Player|GetPlayerPawn 0)))
  (Variables|Default|SetAs%20BP%20Player _asbp_player))

(event Custom|StopShoot
  (Utilities|Time|ClearTimerbyFunctionName 0 "Shooting"))

(event Custom|Shooting
  (bind (_return_value_location _returnvalue) (CallFunction|BulletLocRot))
  (bind _as_bp_player (Variables|Default|GetAs%20BP%20Player))
  (bind _as_abp_player (Variables|/Game/Blueprints/Character/BP_Player.BP_Player_C|GetAs%20ABP%20Player _as_bp_player))
  (if (<= (Variables|Default|GetCurrentAmmoNum) 0)
    (Audio|PlaySound2D "/Game/Sounds/Weapon/AK74/gun_rifle_dry_fire_01_Cue.gun_rifle_dry_fire_01_Cue" 1.0 1.0 0.0 0 0)
    (Utilities|Time|ClearTimerbyFunctionName 0 "Shooting")
    (else
      (Animation|Montage|MontagePlay _as_abp_player (select (Variables|/Game/Blueprints/Character/ABP_Player.ABP_Player_C|GetIsAim _as_abp_player) "/Game/FPS_Assault_Pack/Animations/RU74/A_Arms_RU74_Isight_Shoot01_Montage.A_Arms_RU74_Isight_Shoot01_Montage" "/Game/FPS_Assault_Pack/Animations/RU74/A_Arms_RU74_Shoot02_Montage.A_Arms_RU74_Shoot02_Montage") 1.2 "MontageLength" 0.0 true)
      (Animation|Montage|MontagePlay (Components|SkeletalMesh|GetAnimInstance (Variables|Default|GetSK_RU74_NoAddons)) "/Game/FPS_Assault_Pack/Animations/RU74/A_RU74_Shoot01_Montage.A_RU74_Shoot01_Montage" 2.5 "MontageLength" 0.0 true)
      (Game|SpawnActorfromClass "/Game/Blueprints/Weapon/BP_Bullet.BP_Bullet_C" (Math|Transform|MakeTransform _return_value_location _returnvalue "1.000000,1.000000,1.000000") "AlwaysSpawn" "MultiplyWithRoot" 0 0)
      (bind _result (Math|Integer|DecrementInt (Variables|Default|GetCurrentAmmoNum))
        (:%20%20
          (Development|PrintString (Utilities|String|ToString(Integer) _result))
          (CallFunction|CalcuRecoil))))))

(event Custom|StartShoot
  (Utilities|Time|SetTimerbyFunctionName 0 "Shooting" 0.12 true)
  (CallFunction|Shooting))

(event Custom|StartReload
  (if (> (Variables|Default|GetAllAmmoNum) 0)
    (if (not (== (Variables|Default|GetCurrentAmmoNum) (Variables|Default|GetClipAmmoMaxNum)))
      (if (not (Variables|Default|GetReloading))
        (Variables|Default|SetRemainingAmmoNum (Variables|Default|GetCurrentAmmoNum))
        (Variables|Default|SetCurrentAmmoNum 0)
        (Variables|Default|SetReloading true)
        (Animation|Montage|PlayMontage (Variables|/Script/Engine.Character|GetMesh (Variables|Default|GetAs%20BP%20Player)) (select (<= (Variables|Default|GetRemainingAmmoNum) 0) "/Game/FPS_Assault_Pack/Animations/RU74/A_Arms_RU74_Reload_Empty_Montage.A_Arms_RU74_Reload_Empty_Montage" "/Game/FPS_Assault_Pack/Animations/RU74/A_Arms_RU74_Reload_Montage.A_Arms_RU74_Reload_Montage")
          (:then
            (Animation|Montage|PlayMontage (Variables|Default|GetSK_RU74_NoAddons) (select (<= (Variables|Default|GetRemainingAmmoNum) 0) "/Game/FPS_Assault_Pack/Animations/RU74/A_RU74_Reload_Empty_Montage.A_RU74_Reload_Empty_Montage" "/Game/FPS_Assault_Pack/Animations/RU74/A_RU74_Reload_Montage.A_RU74_Reload_Montage")
              (:OnCompleted
                (Variables|Default|SetReloading false)
                (bind _output_get (Variables|Default|SetCurrentAmmoNum (CallFunction|CalcuRemainingAmmo)))
                (Development|PrintString (Utilities|String|ToString(Integer) _output_get) true true "(R=1.000000,G=0.060870,B=0.000000,A=1.000000)" 25.0)
                (Development|PrintString (Utilities|String|ToString(Integer) (Variables|Default|GetAllAmmoNum)) true true "(R=0.000000,G=0.919867,B=1.000000,A=1.000000)" 25.0)))))))))

(event Custom|CalcuRecoil
  (bind _returnvalue (Game|Player|GetPlayerPawn 0))
  (bind _newtrack_0 (Timeline|Timeline PlayFromStart)
    (:Update
      (Pawn|Input|AddControllerYawInput _returnvalue (Math|Random|RandomFloatinRange -0.2 0.2))
      (Pawn|Input|AddControllerPitchInput _returnvalue (Math|Float|Lerp 0.0 -0.05 _newtrack_0)))))

(fn ConstructionScript)

(fn CalcuRemainingAmmo
  (if (> (- (Variables|Default|GetAllAmmoNum) (- (Variables|Default|GetClipAmmoMaxNum) (Variables|Default|GetRemainingAmmoNum))) 0)
    (Variables|Default|SetAllAmmoNum (- (Variables|Default|GetAllAmmoNum) (- (Variables|Default|GetClipAmmoMaxNum) (Variables|Default|GetRemainingAmmoNum))))
    (Variables|Default|SetRemainingAmmoNum (Variables|Default|GetClipAmmoMaxNum))
    (else
      (Variables|Default|SetRemainingAmmoNum (+ (Variables|Default|GetRemainingAmmoNum) (Variables|Default|GetAllAmmoNum)))
      (Variables|Default|SetAllAmmoNum 0)))
  (return (Variables|Default|GetRemainingAmmoNum)))

(fn BulletLocRot
  (bind _sk_ru74_noaddons (Variables|Default|GetSK_RU74_NoAddons))
  (bind _returnvalue (Transformation|GetSocketTransform _sk_ru74_noaddons "b_MuzzleSocket" "RTS_World"))
  (return (.location _returnvalue) (select (Variables|/Game/Blueprints/Character/ABP_Player.ABP_Player_C|GetIsAim (Variables|/Game/Blueprints/Character/BP_Player.BP_Player_C|GetAs%20ABP%20Player (Variables|Default|GetAs%20BP%20Player))) (.rotation _returnvalue) (Math|Conversions|RotationFromXVector (Math|Random|RandomUnitVectorinConeinDegrees (Math|Rotator|GetRotationXVector (.rotation _returnvalue)) 3.0)))))