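; Zombie enemy that randomizes its mesh, idle and run-or-sprint speed, then chases and melees the player.
; Looping timers drive AI MoveTo and a forward sphere trace that triggers random attack montages.
; Externally triggered bone-to-bone traces apply damage once until reset.
; Damage plays random hit reactions when not attacking; death ragdolls the body, cuts shadow, LOD and movement costs, then destroys it after a delay.
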(event Custom|ChasePlayer
  (bind _returnvalue (Game|Player|GetPlayerPawn 0))
  (AI|AIMoveTo self "0, 0, 0" _returnvalue 1e+02 false
    (:then
      (AI|SetFocus (AI|GetAIController self) _returnvalue))))

(event EventBeginPlay
  (bind _asabp_zombie_enemy (Utilities|Casting|CastToABP_ZombieEnemy (Components|SkeletalMesh|GetAnimInstance (Variables|Character|GetMesh))))
  (Variables|Default|SetAs%20ABP%20Zombie%20Enemy _asabp_zombie_enemy)
  (Utilities|Time|SetTimerbyFunctionName 0 "ChasePlayer" 1.0 true)
  (CallFunction|InitSpeed+Anim)
  (CallFunction|RandomMesh)
  (Utilities|Time|SetTimerbyFunctionName 0 "CheckAttackRange" 0.1 true))

(event Game|Damage|EventAnyDamage
  (params (Damage :type Float%20%28single-precision%29) (DamageType :type Damage%20Type%20Object%20Reference) (InstigatedBy :type Controller%20Object%20Reference) (DamageCauser :type Actor%20Object%20Reference))
  (bind _mesh (Variables|Character|GetMesh))
  (bind _mesh_2 (Variables|Character|GetMesh))
  (bind _output_get (Variables|Default|SetHP (- (Variables|Default|GetHP) Damage)))
  (if (<= _output_get 0.0)
    (Utilities|FlowControl|DoOnce false
      (:Completed
        (Collision|SetCollisionEnabled (Variables|Collision|GetCapsuleComponent) "NoCollision")
        (Physics|SetSimulatePhysics _mesh true)
        (Components|Animation|PlayAnimation _mesh 0 false)
        (Variables|/Script/Engine.CharacterMovementComponent|SetMaxWalkSpeed (Variables|Character|GetCharacterMovement) 0.0)
        (Utilities|FlowControl|Sequence
          (:then_0
            (Utilities|FlowControl|Delay 1e+01)
            (Actor|DestroyActor))
          (:then_1
            (Rendering|SetCastShadow _mesh_2 false)
            (Components|SkinnedMesh|SetForcedLOD _mesh_2 3)
            (Components|DestroyComponent (Variables|Character|GetCharacterMovement))
            (Utilities|Time|ClearTimerbyFunctionName 0 "ChasePlayer")))))
    (elif (not (Variables|Default|GetIsAttacking))
      (if (not (Variables|Default|GetIsRepelling))
        (Variables|Default|SetIsRepelling true)
        (Animation|Montage|PlayMontage (Variables|Character|GetMesh) (Utilities|Select :Index (Math|Random|RandomIntegerinRange 0 2) :Option%200 "/Game/ShirtlessZombiesPack/Zombie_Pack/Animations/InPlace/Hits/Zombie_HitReact_Head_Montage.Zombie_HitReact_Head_Montage" :Option%201 "/Game/ShirtlessZombiesPack/Zombie_Pack/Animations/InPlace/Hits/Zombie_HitReact_LeftArm_Montage.Zombie_HitReact_LeftArm_Montage" :Option%202 "/Game/ShirtlessZombiesPack/Zombie_Pack/Animations/InPlace/Hits/Zombie_HitReact_RightArm_Montage.Zombie_HitReact_RightArm_Montage") 1.3
          (:OnCompleted
            _)
          (:OnInterrupted
            _))
        (Variables|Default|SetIsRepelling false)))))

(event Custom|CheckAttackRange
  (bind _returnvalue (Transformation|GetActorLocation))
  (bind _returnvalue_2 (Collision|SphereTraceByChannel _returnvalue (+ _returnvalue (* (Transformation|GetActorForwardVector) 1.6e+02)) 3e+01 "TraceTypeQuery3" false 0 "None"))
  (if _returnvalue_2
    (if (not (Variables|Default|GetIsAttacking))
      (Variables|Default|SetIsAttacking true)
      (Animation|Montage|PlayMontage (Variables|Character|GetMesh) (Utilities|Select :Index (Math|Random|RandomIntegerinRange 0 3) :Option%200 "/Game/ShirtlessZombiesPack/Zombie_Pack/Animations/InPlace/Attacks/RM_LeftAttack_Charged_02_Montage.RM_LeftAttack_Charged_02_Montage" :Option%201 "/Game/ShirtlessZombiesPack/Zombie_Pack/Animations/InPlace/Attacks/RM_RightAttack_Charged_01_Montage.RM_RightAttack_Charged_01_Montage" :Option%202 "/Game/ShirtlessZombiesPack/Zombie_Pack/Animations/InPlace/Attacks/RM_RightAttack_Charged_02_Montage.RM_RightAttack_Charged_02_Montage" :Option%203 "/Game/ShirtlessZombiesPack/Zombie_Pack/Animations/InPlace/Attacks/RM_RightAttack_Charged_03_Montage.RM_RightAttack_Charged_03_Montage") 1.2
        (:OnCompleted
          (Variables|Default|SetIsAttacking false))))))

(event Custom|CheckAttackDamage
  (bind _mesh (Variables|Character|GetMesh))
  (bind (_outhit _returnvalue) (Collision|SphereTraceByChannel (Transformation|GetSocketLocation _mesh (Variables|Default|GetStartBone)) (Transformation|GetSocketLocation _mesh (Variables|Default|GetEndBone)) 2e+01 "TraceTypeQuery3" false 0 "None"))
  (if _returnvalue
    (Utilities|FlowControl|DoOnce false
      (:Completed
        (Game|Damage|ApplyDamage (.HitActor (Collision|BreakHitResult _outhit)) 1e+01 0 0)
        (Effects|SpawnEmitteratLocation "/Game/Particles/Effects1/SmokeBuilder/Particles/P_SmokePuff1b.P_SmokePuff1b" (.Location (Collision|BreakHitResult _outhit)) (Math|Conversions|RotationFromXVector (.Normal (Collision|BreakHitResult _outhit))) "0.100000,0.100000,0.100000")))))

(event Custom|ResetApplyDamage
  (Utilities|FlowControl|DoOnce false) ; enters at Reset
)

(fn ConstructionScript)

(fn InitSpeed+Anim
  (bind _as_abp_zombie_enemy (Variables|Default|GetAs%20ABP%20Zombie%20Enemy))
  (switch int (Math|Random|RandomIntegerinRange 0 1)
    (:0
      (Variables|/Game/Blueprints/Zombie/ABP_ZombieEnemy.ABP_ZombieEnemy_C|SetMoveAnim _as_abp_zombie_enemy "/Game/ShirtlessZombiesPack/Zombie_Pack/Animations/InPlace/Locomotion/IP_Run_Front.IP_Run_Front")
      (Variables|Default|SetInitSpeed 2e+02))
    (:1
      (Variables|/Game/Blueprints/Zombie/ABP_ZombieEnemy.ABP_ZombieEnemy_C|SetMoveAnim _as_abp_zombie_enemy "/Game/ShirtlessZombiesPack/Zombie_Pack/Animations/InPlace/Locomotion/IP_Sprint_Front.IP_Sprint_Front")
      (Variables|Default|SetInitSpeed 4.8e+02)))
  (Variables|/Game/Blueprints/Zombie/ABP_ZombieEnemy.ABP_ZombieEnemy_C|SetIdleAnim _as_abp_zombie_enemy (Utilities|Select :Index (Math|Random|RandomIntegerinRange 0 2) :Option%200 "/Game/ShirtlessZombiesPack/Zombie_Pack/Animations/InPlace/Idle/IP_Idle_01.IP_Idle_01" :Option%201 "/Game/ShirtlessZombiesPack/Zombie_Pack/Animations/InPlace/Idle/IP_Idle_02.IP_Idle_02" :Option%202 "/Game/ShirtlessZombiesPack/Zombie_Pack/Animations/InPlace/Idle/IP_Idle_08.IP_Idle_08"))
  (Variables|/Game/Blueprints/Zombie/ABP_ZombieEnemy.ABP_ZombieEnemy_C|SetStart%20Position (Variables|Default|GetAs%20ABP%20Zombie%20Enemy) (Math|Random|RandomFloatinRange 0.0 1.0))
  (Variables|/Script/Engine.CharacterMovementComponent|SetMaxWalkSpeed (Variables|Character|GetCharacterMovement) (Variables|Default|GetInitSpeed)))

(fn RandomMesh
  (Components|SkeletalMesh|SetSkeletalMeshAsset (Variables|Character|GetMesh) (Utilities|Select :Index (Math|Random|RandomIntegerinRange 0 4) :Option%200 "/Game/ShirtlessZombiesPack/UE4/SK_ZombieBB_V1.SK_ZombieBB_V1" :Option%201 "/Game/ShirtlessZombiesPack/UE4/SK_ZombieBB_V2.SK_ZombieBB_V2" :Option%202 "/Game/ShirtlessZombiesPack/UE4/SK_ZombieBB_V3.SK_ZombieBB_V3" :Option%203 "/Game/ShirtlessZombiesPack/UE4/SK_ZombieBB_V4.SK_ZombieBB_V4" :Option%204 "/Game/ShirtlessZombiesPack/UE4/SK_ZombieBB_V5.SK_ZombieBB_V5")))